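; Controller Blueprint that loads key icon data and detects switches between keyboard/mouse and gamepad input.
; On BeginPlay it initializes the GeneralSubsystem with keyboard and DualSense data tables, assuming keyboard/mouse as the starting device.
; An AnyKey press, gated by a DoOnce until release, compares the most recently used hardware device to the cached type and notifies GeneralSubsystem of changes.
; GetKeyByAction is an empty stub.
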(event `self.ReceiveBeginPlay`
  ;[1 1 1] Initialize all Keybind Icons in an Array
  (`GeneralSubsystem.InitializeKeyInfo` (subsystem `GeneralSubsystem`) "/Game/InputMapping/UI/KeyBinds/DT_KeyboardKeys.DT_KeyboardKeys" "/Game/InputMapping/UI/KeyBinds/DT_ControllerKeys.DT_ControllerKeys")
  (set `self.Last Primary Device Type` "KeyboardAndMouse"))

(event `Key|AnyKey` :consume false :paused true
  (params (Key :type "Key Structure"))
  (bind _returnvalue (subsystem `GeneralSubsystem`))
  (bind (_inputclassname _hardwaredeviceidentifier _primarydevicetype) (break `HardwareDeviceIdentifier` (`InputDeviceSubsystem.GetMostRecentlyUsedHardwareDevice` :`self` (subsystem `InputDeviceSubsystem`))))
  ;[1 1 1] Check if Input Device is Changed
  (:`Pressed`
    (`/Engine/EditorBlueprintResources/StandardMacros.DoOnce` false :!label _label
      (:`Completed`
        (if (`|EnumEquality` _primarydevicetype (`self.Last Primary Device Type`))
          _
          (elif (`|EnumEquality` "KeyboardAndMouse" _primarydevicetype)
            (set `self.Last Primary Device Type` "KeyboardAndMouse")
            (`GeneralSubsystem.InputDeviceChanged` _returnvalue false)
            (elif (`|EnumEquality` "Gamepad" _primarydevicetype)
              (set `self.Last Primary Device Type` "Gamepad")
              (`GeneralSubsystem.InputDeviceChanged` _returnvalue true)))))))
  (:`Released`
    (goto _label :!via `Reset`)))

(fn `GetKeyByAction`
  (params (Action :type "InputAction Object Reference")))

(fn `UserConstructionScript`)